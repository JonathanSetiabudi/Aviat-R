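; BlackUmbrella is an umbrella prop Blueprint with a tintable panel material and no active runtime logic.
; Its construction script builds a dynamic instance from Shaft001's first material, applies it to Panel001 and stores it as UmbrellaPlastic.
; It then passes a fixed color to SetColor, which writes it to that instance as a vector parameter.
; The parameter name is None, so the tint targets no named material parameter.
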(fn `SetColor`
  (params (Color :type "Color Structure"))
  (`MaterialInstanceDynamic.SetVectorParameterValue` (`self.UmbrellaPlastic`) "None" (`KismetMathLibrary.Conv_ColorToLinearColor` Color)))

(fn `UserConstructionScript`
  (bind _returnvalue (`PrimitiveComponent.CreateDynamicMaterialInstance` (`self.Panel_001`) 0 (`PrimitiveComponent.GetMaterial` (`self.Shaft_001`) 0) "None"))
  (`PrimitiveComponent.SetMaterial` (`self.Panel_001`) 0 _returnvalue)
  (set `self.UmbrellaPlastic` _returnvalue)
  (`self.SetColor` (`KismetMathLibrary.Conv_LinearColorToColor` (make `LinearColor` 0.0))))